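; BP_EndGame is an interactable that ends the game when the interacting actor carries a "Key" in its inventory.
; Interact searches the actor's BPC_Inventory for the key slot, then shows WBP_EndGame and quits after a short delay.
; LookAt puts a WBP_ItemInfo popup describing the object on its Widget, and StopLookat clears it.
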(event EventInteract
  (params (InteractingActor :type Actor%20Object%20Reference))
  ;[1 1 1] Check if the player has the key and end the game
  (bind _foundslot (Default|TryFindSlot (Actor|GetComponentbyClass InteractingActor "/Game/c014004n_StudentWork/01_Blueprints/00_Components/BPC_Inventory.BPC_Inventory_C") "Key"))
  (if _foundslot
    (bind _returnvalue (UserInterface|CreateWidget "/Game/c014004n_StudentWork/08_Widgets/WBP_EndGame.WBP_EndGame_C"))
    (UserInterface|Viewport|AddtoViewport _returnvalue 0)
    (Utilities|FlowControl|Delay 5.0)
    (Game|QuitGame 0 "Quit" false)))

(event EventStopLookat
  ;[1 1 1] Stop showing popup
  (UserInterface|SetWidget (Variables|Default|GetWidget) 0))

(fn ConstructionScript)

(fn Lookat
  ;[1 1 1] Show popup
  (bind _returnvalue (UserInterface|CreateWidget "/Game/c014004n_StudentWork/08_Widgets/SubWidgets/WBP_ItemInfo.WBP_ItemInfo_C" 0 "Will end the game" "Endgame"))
  (UserInterface|SetWidget (Variables|Default|GetWidget) _returnvalue)
  (return ""))