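; BPC_Item is an actor component that turns its owner into an inventory pickup defined by a data table row and quantity.
; Interact passes the item to the interacting actor's BPC_Inventory, then destroys the owner on success or stores the remaining quantity otherwise.
; LookAt looks up the item name in the data table for a "Pick up" prompt.
; LookAtc duplicates LookAt.
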(event EventInteract
  (params (InteractingActor :type Actor%20Object%20Reference))
  (bind _returnvalue (Actor|GetComponentbyClass InteractingActor "/Game/c014004n_StudentWork/01_Blueprints/00_Components/BPC_Inventory.BPC_Inventory_C"))
  (Utilities|IsValid _returnvalue
    (:Is%20Valid
      (bind (_success _quantityremaining) (Default|AddtoInventory _returnvalue (.rowname (Variables|ItemData|GetItemID)) (Variables|ItemData|GetQuantity)))
      (if _success
        (Actor|DestroyActor (Components|GetOwner))
        (else
          (Variables|ItemData|SetQuantity _quantityremaining))))))

(fn LookAtc
  (bind _itemid (Variables|ItemData|GetItemID))
  (bind _returnvalue (Utilities|GetDataTableRow (.datatable _itemid) (.rowname _itemid))
    (:then
      (return (Utilities|Text|FormatText "Pick up {item}" (.ItemName (Utilities|Struct|BreakST_Item _returnvalue)))))))

(fn Lookat
  (bind _itemid (Variables|ItemData|GetItemID))
  (bind _returnvalue (Utilities|GetDataTableRow (.datatable _itemid) (.rowname _itemid))
    (:then
      (return (Utilities|Text|FormatText "Pick up {item}" (.ItemName (Utilities|Struct|BreakST_Item _returnvalue)))))))