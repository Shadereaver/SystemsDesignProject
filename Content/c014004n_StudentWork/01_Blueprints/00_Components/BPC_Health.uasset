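; BPC_Health is a health component that tracks current and maximum health for the player.
; DamageHeal subtracts a signed amount clamped between zero and max health, and reopens MainWorld when health runs out.
; ChangeMaxHealth offsets the maximum without adjusting or re-clamping current health.
; BeginPlay and both functions call CallUpdateHealth with the current values to refresh the HUD.
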(event EventBeginPlay
  ;[1 1 1] Reset hud
  (Default|CallUpdateHealth (Variables|Default|GetCurrentHealth) (Variables|Default|GetMaxHealth)))

(fn Damage/Heal
  (params (Damage :type Float%20%28double-precision%29))
  (bind _maxhealth (Variables|Default|GetMaxHealth))
  ;[1 1 1] Damage/heal the player and check if they died
  (bind _output_get (Variables|Default|SetCurrentHealth (Math|Float|Clamp(Float) (- (Variables|Default|GetCurrentHealth) Damage) 0.0 _maxhealth)))
  (Default|CallUpdateHealth _output_get _maxhealth)
  (if (<= _output_get 0.0)
    (Game|OpenLevel(byName) "MainWorld")))

(fn ChangeMaxHealth
  (params (Change :type Float%20%28double-precision%29))
  ;[1 1 1] Change the max health
  (bind _output_get (Variables|Default|SetMaxHealth (+ Change (Variables|Default|GetMaxHealth))))
  (Default|CallUpdateHealth (Variables|Default|GetCurrentHealth) _output_get))