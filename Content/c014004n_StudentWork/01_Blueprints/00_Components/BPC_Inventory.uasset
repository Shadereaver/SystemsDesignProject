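; BPC_Inventory is an inventory component in which only the look-at and interact behavior is implemented; Add and Remove are empty stubs.
; LookAt caches the passed actor, sends start and stop look-at messages when the target changes or becomes invalid, and prints the returned text as debug output.
; Interact forwards an interact message to that cached actor.
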(fn Add)

(fn Remove)

(fn Lookat
  (params (Actor :type Actor%20Object%20Reference))
  (Utilities|IsValid Actor
    (:Is%20Valid
      (if (!= (Variables|Default|GetLookAtActor) Actor)
        (Class|BPIInteractInterface|StopLookat(Message) (Variables|Default|GetLookAtActor))
        (bind _output_get (Variables|Default|SetLookAtActor Actor))
        (bind _message (Class|BPIInteractInterface|Lookat(Message) _output_get))
        (Development|PrintText _message)))
    (:Is%20Not%20Valid
      (Class|BPIInteractInterface|StopLookat(Message) (Variables|Default|GetLookAtActor))
      (Variables|Default|SetLookAtActor 0)
      (Development|PrintString "Pick up none"))))

(fn Interact
  (Class|BPIInteractInterface|Interact(Message) (Variables|Default|GetLookAtActor)))