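; Actor component that manages food and water survival stats, damaging its owner when either is at zero.
; BeginPlay refreshes the HUD through update calls and starts looping timers that apply each drain amount.
; Gates let either drain be paused, with a one-shot timer reopening it after a given time.
; Change functions clamp current values or adjust maximums, passing results to the update calls.
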(event Custom|FoodDrain
  ;[1 1 1] Allow for the temporary stopping of drain
  (Utilities|FlowControl|Gate false
    (:Exit
      (Food|ChangeFood (Variables|Food|GetFoodDrainAmount)))))

(event Custom|WaterDrain
  ;[1 1 1] Allow for the temporary stopping of drain
  (Utilities|FlowControl|Gate false
    (:Exit
      (Water|ChangeWater (Variables|Water|GetWaterDrainAmount)))))

(event Custom|StartFoodDrain
  ;[1 1 1] Allow for the temporary stopping of drain
  (Utilities|FlowControl|Gate false) ; enters at Open
)

(event Custom|StopWaterDrain
  (params (Time :type Float%20%28double-precision%29))
  ;[1 1 1] Allow for the temporary stopping of drain
  (Utilities|Time|SetTimerbyEvent (delegate Custom|StartWaterDrain) Time)
  (Utilities|FlowControl|Gate false) ; enters at Close
)

(event Custom|StartWaterDrain
  ;[1 1 1] Allow for the temporary stopping of drain
  (Utilities|FlowControl|Gate false) ; enters at Open
)

(event Custom|StopFoodDrain
  (params (Time :type Float%20%28double-precision%29))
  ;[1 1 1] Allow for the temporary stopping of drain
  (Utilities|Time|SetTimerbyEvent (delegate Custom|StartFoodDrain) Time)
  (Utilities|FlowControl|Gate false) ; enters at Close
)

(event EventBeginPlay
  ;[1 1 1] Reset hud to default values
  (Default|CallUpdateFood (Variables|Food|GetCurrrentFood) (Variables|Food|GetMaxFood))
  (Default|CallUpdateWater (Variables|Water|GetCurrentWater) (Variables|Water|GetMaxWater))
  ;[1 1 1] Start timers to drain
  (Utilities|Time|SetTimerbyEvent (EventDispatchers|CreateEvent :!event Custom|FoodDrain) (Variables|Food|GetFoodDrainRate) true)
  (Utilities|Time|SetTimerbyEvent (EventDispatchers|CreateEvent :!event Custom|WaterDrain) (Variables|Water|GetWaterDrainRate) true))

(fn ChangeFood
  (params (Amount :type Float%20%28double-precision%29))
  (bind _maxfood (Variables|Food|GetMaxFood))
  ;[1 1 1] Change the food value by a givent amount and damage the player if zero
  (Default|CallUpdateFood (Math|Float|Clamp(Float) (+ Amount (Variables|Food|GetCurrrentFood)) 0.0 _maxfood) _maxfood)
  (if (<= (Variables|Food|GetCurrrentFood) 0.0)
    (Game|Damage|ApplyDamage (Components|GetOwner) 1e+01 0 0)))

(fn ChangeMaxFood
  (params (Amount :type Float%20%28double-precision%29))
  ;[1 1 1] Change the max food value
  (Default|CallUpdateFood (Variables|Food|GetCurrrentFood) (+ Amount (Variables|Food|GetMaxFood))))

(fn ChangeWater
  (params (Amount :type Float%20%28double-precision%29))
  (bind _maxwater (Variables|Water|GetMaxWater))
  ;[1 1 1] Change the water value by a givent amount and damage the player if zero
  (Default|CallUpdateWater (Math|Float|Clamp(Float) (+ Amount (Variables|Water|GetCurrentWater)) 0.0 _maxwater) _maxwater)
  (if (<= (Variables|Water|GetCurrentWater) 0.0)
    (Game|Damage|ApplyDamage (Components|GetOwner) 1e+01 0 0)))

(fn ChangeMaxWater
  (params (Amount :type Float%20%28double-precision%29))
  ;[1 1 1] Change the max water value
  (Default|CallUpdateWater (Variables|Water|GetCurrentWater) (+ Amount (Variables|Water|GetMaxWater))))