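; BPC_CompassIcon is an actor component that puts an icon for its owning actor on the player's compass.
; On BeginPlay it checks for the player's HUD, retrying on a short non-looping timer until the HUD is valid.
; It then creates a compass icon widget with its icon texture and owner, and adds it to the compass overlay.
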(event Custom|InitialiseIcon
  (params (HUD :type WBP%20Main%20UIHUD%20Object%20Reference))
  ;[1 1 1] Add icon to compass
  (bind _returnvalue (UserInterface|CreateWidget "/Game/c014004n_StudentWork/08_Widgets/SubWidgets/WBP_PlayerCompassIcon.WBP_PlayerCompassIcon_C" 0 (Variables|Compass|GetIcon%20Texture) (Components|GetOwner)))
  (Class|Overlay|AddChildtoOverlay (Variables|/Game/c014004n_StudentWork/08_Widgets/SubWidgets/WBP_PlayerCompass.WBP_PlayerCompass_C|GetOverlay (Variables|/Game/c014004n_StudentWork/08_Widgets/WBP_MainUIHUD.WBP_MainUIHUD_C|GetWBP_PlayerCompass HUD)) _returnvalue))

(event Custom|HUDPoll
  (bind _playerref (CallFunction|GetPlayer))
  (bind _playerhud (Variables|/Game/c014004n_StudentWork/01_Blueprints/BP_Player.BP_Player_C|GetPlayerHUD _playerref))
  ;[1 1 1] Get HUD component if the HUD is not valid set a timer to re-execute the code
  (Utilities|IsValid _playerhud
    (:Is%20Valid
      (CallFunction|InitialiseIcon _playerhud))
    (:Is%20Not%20Valid
      (Utilities|Time|SetTimerbyEvent (delegate Custom|HUDPoll) 0.1))))

(event EventBeginPlay
  (bind _playerref (CallFunction|GetPlayer))
  (bind _playerhud (Variables|/Game/c014004n_StudentWork/01_Blueprints/BP_Player.BP_Player_C|GetPlayerHUD _playerref))
  ;[1 1 1] Get HUD component if the HUD is not valid set a timer to re-execute the code
  (Utilities|IsValid _playerhud
    (:Is%20Valid
      (CallFunction|InitialiseIcon _playerhud))
    (:Is%20Not%20Valid
      (Utilities|Time|SetTimerbyEvent (delegate Custom|HUDPoll) 0.1))))