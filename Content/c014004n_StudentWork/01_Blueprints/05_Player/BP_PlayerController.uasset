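; Player controller that adds the Enhanced Input mapping context and creates the main HUD widget on BeginPlay.
; Gameplay actions are relayed to the controlled pawn as interface messages with their value and event type, with optional look-axis inversion.
; Inventory, pause and map go to the UI, with inventory blocked in build mode.
; Item slot, item scroll and build menu inputs only print debug text.
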(event Input|EnhancedActionEvents|EnhancedInputActionIA_Move
  (params (ActionValue :type Vector%202D%20Structure) (ElapsedSeconds :type Float%20%28double-precision%29) (TriggeredSeconds :type Float%20%28double-precision%29) (InputAction :type Input%20Action%20Object%20Reference :default "/Game/c014004n_StudentWork/03_Input/InputActions/IA_Move.IA_Move"))
  ;[1 1 1] Move interface
  (:Triggered
    (Class|BPIPlayerInterface|IAMove(Message) (Pawn|GetControlledPawn) ActionValue "Triggered")))

(event Input|EnhancedActionEvents|EnhancedInputActionIA_Look
  (params (ActionValue :type Vector%202D%20Structure) (ElapsedSeconds :type Float%20%28double-precision%29) (TriggeredSeconds :type Float%20%28double-precision%29) (InputAction :type Input%20Action%20Object%20Reference :default "/Game/c014004n_StudentWork/03_Input/InputActions/IA_Look.IA_Look"))
  ;[1 1 1] Look interface
  (:Triggered
    (Class|BPIPlayerInterface|IALook(Message) (Pawn|GetControlledPawn) (Math|Vector2D|MakeVector2D (Math|Float|SelectFloat (* (.x ActionValue) -1.0) (.x ActionValue) (Variables|Default|GetbInvertLookX)) (Math|Float|SelectFloat (* (.y ActionValue) -1.0) (.y ActionValue) (Variables|Default|GetbInvertLookY))) "Triggered")))

(event Input|EnhancedActionEvents|EnhancedInputActionIA_Sprint
  (params (ActionValue :type Boolean) (ElapsedSeconds :type Float%20%28double-precision%29) (TriggeredSeconds :type Float%20%28double-precision%29) (InputAction :type Input%20Action%20Object%20Reference :default "/Game/c014004n_StudentWork/03_Input/InputActions/IA_Sprint.IA_Sprint"))
  (bind _returnvalue (Pawn|GetControlledPawn))
  ;[1 1 1] Sprint interface
  (:Triggered
    (Class|BPIPlayerInterface|IASprint(Message) _returnvalue ActionValue "Triggered"))
  (:Completed
    (Class|BPIPlayerInterface|IASprint(Message) _returnvalue ActionValue "Completed")))

(event Input|EnhancedActionEvents|EnhancedInputActionIA_Roll
  (params (ActionValue :type Boolean) (ElapsedSeconds :type Float%20%28double-precision%29) (TriggeredSeconds :type Float%20%28double-precision%29) (InputAction :type Input%20Action%20Object%20Reference :default "/Game/c014004n_StudentWork/03_Input/InputActions/IA_Roll.IA_Roll"))
  ;[1 1 1] Roll interface
  (:Triggered
    (Class|BPIPlayerInterface|IARoll(Message) (Pawn|GetControlledPawn) ActionValue "Triggered")))

(event Input|EnhancedActionEvents|EnhancedInputActionIA_ItemSlot
  (params (ActionValue :type Float%20%28double-precision%29) (ElapsedSeconds :type Float%20%28double-precision%29) (TriggeredSeconds :type Float%20%28double-precision%29) (InputAction :type Input%20Action%20Object%20Reference :default "/Game/c014004n_StudentWork/03_Input/InputActions/IA_ItemSlot.IA_ItemSlot"))
  ;[1 1 1] Numberkey select
  (:Triggered
    (Development|PrintString (Utilities|String|Append "Slot: " (Utilities|String|ToString(Integer) (Class|KismetMathLibrary|FTrunc64 ActionValue))))))

(event Input|EnhancedActionEvents|EnhancedInputActionIA_ItemScroll
  (params (ActionValue :type Float%20%28double-precision%29) (ElapsedSeconds :type Float%20%28double-precision%29) (TriggeredSeconds :type Float%20%28double-precision%29) (InputAction :type Input%20Action%20Object%20Reference :default "/Game/c014004n_StudentWork/03_Input/InputActions/IA_ItemScroll.IA_ItemScroll"))
  ;[1 1 1] Item select
  (:Triggered
    (bind _bbuildmode (Class|BPIPlayerInterface|IsBuildMode(Message) (Pawn|GetControlledPawn)))
    (if (not _bbuildmode)
      (Development|PrintString (Utilities|String|Append "Item scroll: " (Utilities|String|ToString(Float) ActionValue))))))

(event Input|EnhancedActionEvents|EnhancedInputActionIA_Aim
  (params (ActionValue :type Boolean) (ElapsedSeconds :type Float%20%28double-precision%29) (TriggeredSeconds :type Float%20%28double-precision%29) (InputAction :type Input%20Action%20Object%20Reference :default "/Game/c014004n_StudentWork/03_Input/InputActions/IA_Aim.IA_Aim"))
  ;[1 1 1] Aim interface
  (:Triggered
    (Class|BPIPlayerInterface|IAAim(Message) (Pawn|GetControlledPawn) ActionValue "Triggered")))

(event Input|EnhancedActionEvents|EnhancedInputActionIA_Attack
  (params (ActionValue :type Boolean) (ElapsedSeconds :type Float%20%28double-precision%29) (TriggeredSeconds :type Float%20%28double-precision%29) (InputAction :type Input%20Action%20Object%20Reference :default "/Game/c014004n_StudentWork/03_Input/InputActions/IA_Attack.IA_Attack"))
  ;[1 1 1] Attack interface
  (:Triggered
    (Class|BPIPlayerInterface|IAAttack(Message) (Pawn|GetControlledPawn) ActionValue "Triggered")))

(event Input|EnhancedActionEvents|EnhancedInputActionIA_Build
  (params (ActionValue :type Boolean) (ElapsedSeconds :type Float%20%28double-precision%29) (TriggeredSeconds :type Float%20%28double-precision%29) (InputAction :type Input%20Action%20Object%20Reference :default "/Game/c014004n_StudentWork/03_Input/InputActions/IA_Build.IA_Build"))
  ;[1 1 1] Build interface
  (:Triggered
    (Class|BPIPlayerInterface|IABuild(Message) (Pawn|GetControlledPawn) ActionValue "Triggered")))

(event Input|EnhancedActionEvents|EnhancedInputActionIA_Deconstruct
  (params (ActionValue :type Boolean) (ElapsedSeconds :type Float%20%28double-precision%29) (TriggeredSeconds :type Float%20%28double-precision%29) (InputAction :type Input%20Action%20Object%20Reference :default "/Game/c014004n_StudentWork/03_Input/InputActions/IA_Deconstruct.IA_Deconstruct"))
  ;[1 1 1] Deconstruct interface
  (:Triggered
    (Class|BPIPlayerInterface|IADeconstruct(Message) (Pawn|GetControlledPawn) ActionValue "Triggered")))

(event Input|EnhancedActionEvents|EnhancedInputActionIA_BuildMode
  (params (ActionValue :type Boolean) (ElapsedSeconds :type Float%20%28double-precision%29) (TriggeredSeconds :type Float%20%28double-precision%29) (InputAction :type Input%20Action%20Object%20Reference :default "/Game/c014004n_StudentWork/03_Input/InputActions/IA_BuildMode.IA_BuildMode"))
  ;[1 1 1] Build mode interface
  (:Triggered
    (Class|BPIPlayerInterface|IABuildMode(Message) (Pawn|GetControlledPawn) ActionValue "Triggered")))

(event Input|EnhancedActionEvents|EnhancedInputActionIA_Rotate
  (params (ActionValue :type Float%20%28double-precision%29) (ElapsedSeconds :type Float%20%28double-precision%29) (TriggeredSeconds :type Float%20%28double-precision%29) (InputAction :type Input%20Action%20Object%20Reference :default "/Game/c014004n_StudentWork/03_Input/InputActions/IA_Rotate.IA_Rotate"))
  ;[1 1 1] Rotate interface
  (:Triggered
    (Class|BPIPlayerInterface|IARotate(Message) (Pawn|GetControlledPawn) ActionValue "Triggered")))

(event Input|EnhancedActionEvents|EnhancedInputActionIA_Jump
  (params (ActionValue :type Boolean) (ElapsedSeconds :type Float%20%28double-precision%29) (TriggeredSeconds :type Float%20%28double-precision%29) (InputAction :type Input%20Action%20Object%20Reference :default "/Game/c014004n_StudentWork/03_Input/InputActions/IA_Jump.IA_Jump"))
  (bind _returnvalue (Pawn|GetControlledPawn))
  ;[1 1 1] Jump interface
  (:Triggered
    (Class|BPIPlayerInterface|IAJump(Message) _returnvalue ActionValue "Triggered"))
  (:Completed
    (Class|BPIPlayerInterface|IAJump(Message) _returnvalue ActionValue "Completed")))

(event Input|EnhancedActionEvents|EnhancedInputActionIA_Undo
  (params (ActionValue :type Boolean) (ElapsedSeconds :type Float%20%28double-precision%29) (TriggeredSeconds :type Float%20%28double-precision%29) (InputAction :type Input%20Action%20Object%20Reference :default "/Game/c014004n_StudentWork/03_Input/InputActions/IA_Undo.IA_Undo"))
  ;[1 1 1] Undo interface
  (:Triggered
    (Class|BPIPlayerInterface|IAUndo(Message) (Pawn|GetControlledPawn) ActionValue "Triggered")))

(event Input|EnhancedActionEvents|EnhancedInputActionIA_Focus
  (params (ActionValue :type Boolean) (ElapsedSeconds :type Float%20%28double-precision%29) (TriggeredSeconds :type Float%20%28double-precision%29) (InputAction :type Input%20Action%20Object%20Reference :default "/Game/c014004n_StudentWork/03_Input/InputActions/IA_Focus.IA_Focus"))
  (bind _returnvalue (Pawn|GetControlledPawn))
  ;[1 1 1] Focus interface
  (:Started
    (Class|BPIPlayerInterface|IAFocus(Message) _returnvalue ActionValue "Started"))
  (:Completed
    (Class|BPIPlayerInterface|IAFocus(Message) _returnvalue ActionValue "Completed")))

(event Input|EnhancedActionEvents|EnhancedInputActionIA_Ping
  (params (ActionValue :type Boolean) (ElapsedSeconds :type Float%20%28double-precision%29) (TriggeredSeconds :type Float%20%28double-precision%29) (InputAction :type Input%20Action%20Object%20Reference :default "/Game/c014004n_StudentWork/03_Input/InputActions/IA_Ping.IA_Ping"))
  ;[1 1 1] Ping interface
  (:Triggered
    (Class|BPIPlayerInterface|IAPing(Message) (Pawn|GetControlledPawn) ActionValue "Triggered")))

(event Input|EnhancedActionEvents|EnhancedInputActionIA_Prone
  (params (ActionValue :type Boolean) (ElapsedSeconds :type Float%20%28double-precision%29) (TriggeredSeconds :type Float%20%28double-precision%29) (InputAction :type Input%20Action%20Object%20Reference :default "/Game/c014004n_StudentWork/03_Input/InputActions/IA_Prone.IA_Prone"))
  ;[1 1 1] Prone interface
  (:Triggered
    (Class|BPIPlayerInterface|IAProne(Message) (Pawn|GetControlledPawn) ActionValue "Triggered")))

(event Input|EnhancedActionEvents|EnhancedInputActionIA_Map
  (params (ActionValue :type Boolean) (ElapsedSeconds :type Float%20%28double-precision%29) (TriggeredSeconds :type Float%20%28double-precision%29) (InputAction :type Input%20Action%20Object%20Reference :default "/Game/c014004n_StudentWork/03_Input/InputActions/IA_Map.IA_Map"))
  ;[1 1 1] Map
  (:Triggered
    (Class|BPIUIInterface|Map(Message) (Variables|Default|GetUI))))

(event Input|EnhancedActionEvents|EnhancedInputActionIA_OpenBuildMenu
  (params (ActionValue :type Boolean) (ElapsedSeconds :type Float%20%28double-precision%29) (TriggeredSeconds :type Float%20%28double-precision%29) (InputAction :type Input%20Action%20Object%20Reference :default "/Game/c014004n_StudentWork/03_Input/InputActions/IA_OpenBuildMenu.IA_OpenBuildMenu"))
  ;[1 1 1] Build menu
  (:Triggered
    (bind _bbuildmode (Class|BPIPlayerInterface|IsBuildMode(Message) (Pawn|GetControlledPawn)))
    (if _bbuildmode
      (Development|PrintString "Build menu"))))

(event Input|EnhancedActionEvents|EnhancedInputActionIA_Interact
  (params (ActionValue :type Boolean) (ElapsedSeconds :type Float%20%28double-precision%29) (TriggeredSeconds :type Float%20%28double-precision%29) (InputAction :type Input%20Action%20Object%20Reference :default "/Game/c014004n_StudentWork/03_Input/InputActions/IA_Interact.IA_Interact"))
  ;[1 1 1] Interact interface
  (:Triggered
    (Class|BPIPlayerInterface|IAInteract(Message) (Pawn|GetControlledPawn) ActionValue "Triggered")))

(event Input|EnhancedActionEvents|EnhancedInputActionIA_Crouch
  (params (ActionValue :type Boolean) (ElapsedSeconds :type Float%20%28double-precision%29) (TriggeredSeconds :type Float%20%28double-precision%29) (InputAction :type Input%20Action%20Object%20Reference :default "/Game/c014004n_StudentWork/03_Input/InputActions/IA_Crouch.IA_Crouch"))
  (bind _returnvalue (Pawn|GetControlledPawn))
  ;[1 1 1] Crouch interface
  (:Started
    (Class|BPIPlayerInterface|IACrouch(Message) _returnvalue ActionValue "Started"))
  (:Completed
    (Class|BPIPlayerInterface|IACrouch(Message) _returnvalue ActionValue "Started")))

(event Input|EnhancedActionEvents|EnhancedInputActionIA_CrouchToggle
  (params (ActionValue :type Boolean) (ElapsedSeconds :type Float%20%28double-precision%29) (TriggeredSeconds :type Float%20%28double-precision%29) (InputAction :type Input%20Action%20Object%20Reference :default "/Game/c014004n_StudentWork/03_Input/InputActions/IA_CrouchToggle.IA_CrouchToggle"))
  ;[1 1 1] Crouch interface
  (:Triggered
    (Class|BPIPlayerInterface|IACrouchToggle(Message) (Pawn|GetControlledPawn) ActionValue "Triggered")))

(event Input|EnhancedActionEvents|EnhancedInputActionIA_Inventory
  (params (ActionValue :type Boolean) (ElapsedSeconds :type Float%20%28double-precision%29) (TriggeredSeconds :type Float%20%28double-precision%29) (InputAction :type Input%20Action%20Object%20Reference :default "/Game/c014004n_StudentWork/03_Input/InputActions/IA_Inventory.IA_Inventory"))
  ;[1 1 1] Inventory
  (:Triggered
    (bind _bbuildmode (Class|BPIPlayerInterface|IsBuildMode(Message) (Pawn|GetControlledPawn)))
    (if (not _bbuildmode)
      (Class|BPIUIInterface|Inventory(Message) (Variables|Default|GetUI)))))

(event Input|EnhancedActionEvents|EnhancedInputActionIA_SprintToggle
  (params (ActionValue :type Boolean) (ElapsedSeconds :type Float%20%28double-precision%29) (TriggeredSeconds :type Float%20%28double-precision%29) (InputAction :type Input%20Action%20Object%20Reference :default "/Game/c014004n_StudentWork/03_Input/InputActions/IA_SprintToggle.IA_SprintToggle"))
  ;[1 1 1] Sprint interface
  (:Triggered
    (Class|BPIPlayerInterface|IASprintToggle(Message) (Pawn|GetControlledPawn) ActionValue "Triggered")))

(event Input|EnhancedActionEvents|EnhancedInputActionIA_Pause
  (params (ActionValue :type Boolean) (ElapsedSeconds :type Float%20%28double-precision%29) (TriggeredSeconds :type Float%20%28double-precision%29) (InputAction :type Input%20Action%20Object%20Reference :default "/Game/c014004n_StudentWork/03_Input/InputActions/IA_Pause.IA_Pause"))
  ;[1 1 1] Pause
  (:Triggered
    (Class|BPIUIInterface|Pause/Resume(Message) (Variables|Default|GetUI))))

(event EventBeginPlay
  (bind _self self)
  (bind _returnvalue (PlayerController|LocalPlayerSubsystems|GetEnhancedInputLocalPlayerSubsystem _self))
  ;[1 1 1] Add player input
  (Utilities|IsValid _returnvalue
    (:Is%20Valid
      (Input|AddMappingContext _returnvalue "/Game/c014004n_StudentWork/03_Input/IMC_DefualtPlayerInput.IMC_DefualtPlayerInput" 0 "(bIgnoreAllPressedKeysUntilRelease=True,bForceImmediately=False)")
      ;[1 1 1] Add hud to player
      (bind _returnvalue_2 (UserInterface|CreateWidget "/Game/c014004n_StudentWork/08_Widgets/WBP_MainUI.WBP_MainUI_C"))
      (bind _output_get (Variables|Default|SetUI _returnvalue_2))
      (UserInterface|Viewport|AddtoViewport _output_get 0)
      (Class|BPIUIInterface|Init(Message) _output_get))))

(fn ConstructionScript)

(fn GetUI
  (return (Variables|Default|GetUI)))