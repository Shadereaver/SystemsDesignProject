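; BP_EnemyBase is an enemy base Blueprint that provides an attack dealing damage to a given target within close range.
; The Attack event runs a multi-sphere trace centered on the actor, then applies fixed damage to the first hit matching the target and stops.
; GetStartAndEndPoint only returns start and end values and is not used by the attack, and the construction script is empty.
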(event EventAttack
  (params (TargetActor :type Actor%20Object%20Reference))
  (bind _returnvalue (Transformation|GetActorLocation))
  ;[1 1 1] Attack the player when in range
  (bind (_outhits _returnvalue_2) (Collision|MultiSphereTraceByChannel _returnvalue _returnvalue 2e+02 "TraceTypeQuery4" false 0 "None"))
  (if _returnvalue_2
    (bind _array_element (Utilities|Array|ForEachLoopwithBreak _outhits :!label _label)
      (:LoopBody
        (if (== TargetActor (.HitActor (Collision|BreakHitResult _array_element)))
          (Game|Damage|ApplyDamage (.HitActor (Collision|BreakHitResult _array_element)) 1e+01 0 0)
          (goto _label Break))))))

(fn ConstructionScript)

(fn GetStartandEndPoint
  (return (Variables|Default|GetStart) (Variables|Default|GetEnd)))