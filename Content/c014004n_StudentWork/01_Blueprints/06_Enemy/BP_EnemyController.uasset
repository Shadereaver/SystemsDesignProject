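; AI controller for an enemy that runs the BT_EnemyBasic behavior tree and seeds its blackboard with an attack radius and the pawn's start and end points.
; Perception updates are routed by sense through a SenseCheck macro.
; Sight sets the player as target and clears the point of interest, or clears the target otherwise.
; Hearing stores the noise location as the point of interest, and invalid targets are cleared.
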(event OnTargetPerceptionUpdated(AIPerception)
  (params (Actor :type Actor%20Object%20Reference) (Stimulus :type AI%20Stimulus%20Structure))
  ;[1 1 1] AI perception handlling
  (bind _returnvalue (Class|AIPerceptionSystem|GetSenseClassforStimulus Stimulus))
  (Utilities|SenseCheck _returnvalue
    (:Sight
      (CallFunction|SightPerception Actor Stimulus))
    (:Sound
      (CallFunction|SoundPerception Stimulus))))

(event OnTargetPerceptionInfoUpdated(AIPerception)
  (params (UpdateInfo :type Actor%20Perception%20Update%20Info%20Structure%20%28by%20ref%29))
  ;[1 1 1] AI perception handlling
  (Utilities|IsValid (Utilities|Struct|BreakActorPerceptionUpdateInfo UpdateInfo)
    (:Is%20Not%20Valid
      (AI|Components|Blackboard|ClearValue (AI|GetBlackboard 0) (Variables|Blackboardkeys|GetTargetActorKey)))))

(event EventBeginPlay
  (bind _returnvalue (AI|GetBlackboard 0))
  ;[1 1 1] Start behaviour tree and pass in values
  (AI|RunBehaviorTree "/Game/c014004n_StudentWork/10_BehaviorTrees/BT_EnemyBasic.BT_EnemyBasic")
  (AI|Components|Blackboard|SetValueasFloat _returnvalue (Variables|Blackboardkeys|GetAttackRadiusKey) 3e+02)
  (bind (_start _end) (Class|BPIEnemy|GetStartandEndPoint(Message) (Pawn|GetControlledPawn)))
  (AI|Components|Blackboard|SetValueasObject _returnvalue (Variables|Blackboardkeys|GetStartKey) _start)
  (AI|Components|Blackboard|SetValueasObject _returnvalue (Variables|Blackboardkeys|GetEndKey) _end))

(fn ConstructionScript)

(fn SightPerception
  (params (InputPin :type Actor%20Object%20Reference) (AIStimulus :type AI%20Stimulus%20Structure%20%28by%20ref%29))
  (bind _returnvalue (AI|GetBlackboard 0))
  (bind _targetactorkey (Variables|Blackboardkeys|GetTargetActorKey))
  ;[1 1 1] Handle sight perception
  (if (and (Utilities|Struct|BreakAIStimulus AIStimulus) (== InputPin (Game|Player|GetPlayerPawn 0)))
    (AI|Components|Blackboard|SetValueasObject _returnvalue _targetactorkey InputPin)
    (AI|Components|Blackboard|ClearValue (AI|GetBlackboard 0) (Variables|Blackboardkeys|GetPOIKey))
    (else
      (AI|Components|Blackboard|ClearValue _returnvalue _targetactorkey))))

(fn SoundPerception
  (params (AIStimulus :type AI%20Stimulus%20Structure%20%28by%20ref%29))
  (bind (_stimuluslocation _bsuccessfullysensed) (Utilities|Struct|BreakAIStimulus AIStimulus))
  ;[1 1 1] Handle sound perception
  (if _bsuccessfullysensed
    (AI|Components|Blackboard|SetValueasVector (AI|GetBlackboard 0) (Variables|Blackboardkeys|GetPOIKey) _stimuluslocation)))