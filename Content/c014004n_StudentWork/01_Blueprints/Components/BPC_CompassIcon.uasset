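; BPC_CompassIcon is a component that adds an icon for its owning actor to the player's compass.
; On BeginPlay it gets the HUD through a player reference message on the player character, retrying on a short timer until that HUD is valid.
; It then creates a compass icon widget, passing its texture and owner, and adds it to the compass overlay.
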(event Custom|InitialiseIcon
  (params (HUD :type WBP%20Main%20UIHUD%20Object%20Reference))
  ;[1 1 1] Add icon to compass
  (bind _returnvalue (UserInterface|CreateWidget "/Game/c014004n_StudentWork/08_UI/WBP_PlayerCompassIcon.WBP_PlayerCompassIcon_C" 0 (Variables|Compass|GetIcon%20Texture) (Components|GetOwner)))
  (Class|Overlay|AddChildtoOverlay (Variables|/Game/c014004n_StudentWork/08_UI/WBP_PlayerCompass.WBP_PlayerCompass_C|GetOverlay (Variables|/Game/c014004n_StudentWork/08_UI/WBP_MainUIHUD.WBP_MainUIHUD_C|GetWBP_PlayerCompass HUD)) _returnvalue))

(event Custom|HUDPoll
  ;[1 1 1] Get HUD component if the HUD is not valid set a timer to re-execute the code
  (bind _playerref (Class|BPIPlayerInterface|GetPlayerRef(Message) (Game|GetPlayerCharacter 0)))
  (Utilities|IsValid (Variables|/Game/c014004n_StudentWork/01_Blueprints/BP_Player.BP_Player_C|GetPlayerHUD _playerref)
    (:Is%20Valid
      (CallFunction|InitialiseIcon (Variables|/Game/c014004n_StudentWork/01_Blueprints/BP_Player.BP_Player_C|GetPlayerHUD _playerref)))
    (:Is%20Not%20Valid
      (Utilities|Time|SetTimerbyEvent (delegate Custom|HUDPoll) 0.1))))

(event EventBeginPlay
  ;[1 1 1] Get HUD component if the HUD is not valid set a timer to re-execute the code
  (bind _playerref (Class|BPIPlayerInterface|GetPlayerRef(Message) (Game|GetPlayerCharacter 0)))
  (Utilities|IsValid (Variables|/Game/c014004n_StudentWork/01_Blueprints/BP_Player.BP_Player_C|GetPlayerHUD _playerref)
    (:Is%20Valid
      (CallFunction|InitialiseIcon (Variables|/Game/c014004n_StudentWork/01_Blueprints/BP_Player.BP_Player_C|GetPlayerHUD _playerref)))
    (:Is%20Not%20Valid
      (Utilities|Time|SetTimerbyEvent (delegate Custom|HUDPoll) 0.1))))